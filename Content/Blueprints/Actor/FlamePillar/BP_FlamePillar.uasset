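; BP_FlamePillar is a flame pillar actor whose light flickers continuously.
; BeginPlay waits a short random delay, likely so separate pillars fall out of sync, then starts one of two flame timelines at random.
; Each timeline scales FlameLight intensity by BaseFlameIntesity through its curve and, when finished, picks a random timeline again, giving an endless irregular flicker.
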(event `PlayRandomFlameTimeline`
  ;[1 1 1] Play Random Timeline
  (if (>= (`KismetMathLibrary.RandomInteger` 2) 1)
    (`self.PlayFlameTimeline1`)
    (else
      (`self.PlayFlameTimeline2`))))

(event `PlayFlameTimeline1`
  ;[1 1 1] Flame Timeline 1
  (bind (_direction _flameintesity) (`Timeline|FlameTimeline1` :!via `PlayFromStart`)
    (:`Update`
      (`LightComponent.SetIntensity` (`self.FlameLight`) (* _flameintesity (`self.BaseFlameIntesity`))))
    (:`Finished`
      (`self.PlayRandomFlameTimeline`))))

(event `PlayFlameTimeline2`
  ;[1 1 1] Flame Timeline 2
  (bind (_direction _flameintesity2) (`Timeline|FlameTimeline2` :!via `PlayFromStart`)
    (:`Update`
      (`LightComponent.SetIntensity` (`self.FlameLight`) (* _flameintesity2 (`self.BaseFlameIntesity`))))
    (:`Finished`
      (`self.PlayRandomFlameTimeline`))))

(event `self.ReceiveBeginPlay`
  (`KismetSystemLibrary.Delay` (`KismetMathLibrary.RandomFloatInRange` 0.1 1.0))
  (`self.PlayRandomFlameTimeline`))

(fn `UserConstructionScript`)