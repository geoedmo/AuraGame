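; GA_Firebolt is the Firebolt gameplay ability, which casts a projectile toward the point under the mouse cursor.
; It gets the target location from mouse target data, turns the avatar to face it through the CombatInterface, and plays the cast montage.
; The montage's FireBolt gameplay event triggers the projectile spawn, and the ability ends after a short delay.
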(event `self.K2_ActivateAbility`
  (bind (_asynctaskproxy _data) (`TargetDataUnderMouse.CreateTargetDataUnderMouse`)
    (:`ValidData`
      (set `self.ProjectTargetLocation` (`.Location` (`GameplayStatics.BreakHitResult` (`AbilitySystemBlueprintLibrary.GetHitResultFromTargetData` _data))))
      (bind _ascombat_interface (cast `CombatInterface` (`self.GetAvatarActorFromActorInfo`)))
      (`CombatInterface.UpdateFacingTarget` _ascombat_interface (`self.ProjectTargetLocation`))
      (`AbilityTask_PlayMontageAndWait.CreatePlayMontageAndWaitProxy` "None" "/Game/Assets/Characters/Aura/Animations/Abilities/AM_Cast_Firebolt.AM_Cast_Firebolt"
        (:`then`
          (`AbilityTask_WaitGameplayEvent.WaitGameplayEvent` (struct :`TagName` "Event.Montage.FireBolt") null
            (:`EventReceived`
              (`self.SpawnProjectile` (`self.ProjectTargetLocation`))
              (`KismetSystemLibrary.Delay` 0.2)
              (`self.K2_EndAbility`))))))))