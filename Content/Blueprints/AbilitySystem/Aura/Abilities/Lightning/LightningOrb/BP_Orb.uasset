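; BP_Orb is the Lightning Orb ability's actor, which periodically seeks nearby players and links electricity splines to them.
; On BeginPlay it runs the search immediately and starts a looping timer at SearchFrequency.
; Each pass calls SeekNearByPlayers, then prints the name of each result and calls SpawnElectrictySplineAttachedToActor on it.
; The timer is cleared when the orb is destroyed.
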(event `self.ReceiveBeginPlay`
  (bind _returnvalue (`KismetSystemLibrary.K2_SetTimerDelegate` (delegate `AttackNearByPlayers`) (`self.SearchFrequency`) true))
  (set `self.AttackNearByPlayersTimer` _returnvalue)
  (`self.AttackNearByPlayers`))

(event `AttackNearByPlayers`
  (bind _returnvalue (`self.SeekNearByPlayers`))
  (for _array_element _returnvalue
    (`KismetSystemLibrary.PrintString` (`KismetSystemLibrary.GetDisplayName` _array_element))
    (`self.SpawnElectrictySplineAttachedToActor` _array_element)))

(event `self.ReceiveDestroyed`
  (`KismetSystemLibrary.K2_ClearAndInvalidateTimerHandle` (`self.AttackNearByPlayersTimer`)))

(event `self.ReceiveTick`
  (params (DeltaSeconds :type "Float (single-precision)")))

(fn `UserConstructionScript`)