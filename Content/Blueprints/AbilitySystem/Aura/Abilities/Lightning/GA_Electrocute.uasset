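; Aura's Electrocute ability: a channeled lightning cast aimed under the mouse that lasts until input is released.
; It stores the hit, faces the target, plays a montage and waits on cast completion to enter the shock loop and trace from the weapon.
; The beam is a looping gameplay cue on the combat target or caster; additional chain targets are only debug-drawn.
; Release removes cues and restores cursor and walking.
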(event `self.K2_ActivateAbility`
  (`self.BP_ApplyGameplayEffectToOwner` "/Game/Blueprints/AbilitySystem/Aura/Abilities/Lightning/GE_ShockCast.GE_ShockCast_C")
  (`self.EnforceActorImplementsInterface`)
  ;[0.2663 0.2359 1] Store Mouse Data
  (bind (_asynctaskproxy _data) (`TargetDataUnderMouse.CreateTargetDataUnderMouse`)
    (:`ValidData`
      (`self.StoreMouseInfoData` (`AbilitySystemBlueprintLibrary.GetHitResultFromTargetData` _data))
      (`self.StoreOwnerVariables`)
      (`|ExecutionSequence`
        (:`then_0`
          (set `PlayerController.bShowMouseCursor` false (`self.StoredOwnerController`))
          (`self.UpdateFacingTarget`)
          (`AbilityTask_PlayMontageAndWait.CreatePlayMontageAndWaitProxy` "None" (`self.Montage_Electrocute`)
            (:`then`
              (`WaitCastTimeChange.WaitForCastCompletion` (`self.GetAbilitySystemComponentFromActorInfo`)
                (:`then`
                  (`self.InShockLoop`))
                (:`CastTimeEnd`
                  (`self.CastElectrocute`))))))
        (:`then_1`
          (`AbilityTask_WaitInputRelease.WaitInputRelease` false
            (:`OnRelease`
              (`self.PrepareToEndAbility`)
              (`self.K2_EndAbility`))))))))

(fn `CastElectrocute`
  (locals (Weapon :type "SkeletalMeshComponent Object Reference"))
  (`self.PerformFirstTraceFromWeapon`)
  (`self.K2_ExecuteGameplayCue` (struct :`TagName` "GameplayCue.ShockNoify"))
  (bind _returnvalue (message `CombatInterface.GetWeapon` (`self.GetAvatarActorFromActorInfo`)))
  (set `local.Weapon` _returnvalue)
  (set `self.FirstCueParams` (`AbilitySystemBlueprintLibrary.MakeGameplayCueParameters` 0.0 0.0 (struct) (struct) (struct) (struct) (struct) (`self.MouseHitLocation`) (0.0 0.0 0.0) null null (`self.MouseHitActor`) null 1 1 (`local.Weapon`)))
  ;[1 1 1] Mouse Hit Actor Implements Combat interface
  (bind _output_get (set `self.bFirstTargetImplementsCombatInterface` (`KismetSystemLibrary.DoesImplementInterface` (`self.MouseHitActor`) "/Script/Aura.CombatInterface")))
  (if _output_get
    (set `self.CueTarget` (`self.MouseHitActor`))
    (`GameplayCueFunctionLibrary.AddGameplayCueOnActor` (`self.CueTarget`) (struct :`TagName` "GameplayCue.ShockLoop") (`self.FirstCueParams`))
    (bind _outadditionaltargets (`self.StoreAdditionalTargets`))
    (`KismetSystemLibrary.DrawDebugSphere` (`self.MouseHitLocation`) 850.0 12 (struct :`R` 1.0 :`G` 1.0 :`B` 1.0 :`A` 1.0) 5.0 1.0)
    (for _array_element _outadditionaltargets
      (`KismetSystemLibrary.PrintString` (`KismetSystemLibrary.GetDisplayName` _array_element) true true (struct :`G` 0.66 :`B` 1.0 :`A` 1.0) 5.0)
      (`KismetSystemLibrary.DrawDebugSphere` (`Actor.K2_GetActorLocation` _array_element) 25.0 12 (struct :`R` 1.0 :`A` 1.0) 5.0))
    (else
      (set `self.CueTarget` (`self.GetAvatarActorFromActorInfo`))
      (`GameplayCueFunctionLibrary.AddGameplayCueOnActor` (`self.CueTarget`) (struct :`TagName` "GameplayCue.ShockLoop") (`self.FirstCueParams`))
      (`CharacterMovementComponent.DisableMovement` (`Character.CharacterMovement` (`self.StoredOwnerCharacter`))))))

(fn `EnforceActorImplementsInterface`
  (if (not (`KismetSystemLibrary.DoesImplementInterface` (`self.GetAvatarActorFromActorInfo`) "/Script/Aura.CombatInterface"))
    (`self.K2_EndAbility`)))

(fn `InShockLoop`
  (message `CombatInterface.SetIsShocking` (`self.GetAvatarActorFromActorInfo`) true))

(fn `PrepareToEndAbility`
  (message `CombatInterface.SetIsShocking` (`self.GetAvatarActorFromActorInfo`) false)
  (set `PlayerController.bShowMouseCursor` true (`self.StoredOwnerController`))
  (`self.K2_RemoveGameplayCue` (struct :`TagName` "GameplayCue.ShockNoify"))
  (`CharacterMovementComponent.SetMovementMode` (`Character.CharacterMovement` (`self.StoredOwnerCharacter`)) "MOVE_Walking" 0)
  (if (`self.bFirstTargetImplementsCombatInterface`)
    (`GameplayCueFunctionLibrary.RemoveGameplayCueOnActor` (`self.MouseHitActor`) (struct :`TagName` "GameplayCue.ShockLoop") (`self.FirstCueParams`))
    (else
      (`GameplayCueFunctionLibrary.RemoveGameplayCueOnActor` (`self.GetAvatarActorFromActorInfo`) (struct :`TagName` "GameplayCue.ShockLoop") (`self.FirstCueParams`)))))

(fn `UpdateFacingTarget`
  (message `CombatInterface.UpdateFacingTarget` (`self.GetAvatarActorFromActorInfo`) (`self.MouseHitLocation`)))