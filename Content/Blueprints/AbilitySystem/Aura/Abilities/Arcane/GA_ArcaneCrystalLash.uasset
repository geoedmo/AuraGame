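; Aura's Arcane Crystal Lash ability, a spinning dash along a line of spawned crystals.
; While input is held it shows a travel arrow; on release it takes the arrow's point, plays the spin montage and sound, and calls SpawnCrystals.
; It boosts walk speed and acceleration, ignores move input and uses SimpleMoveToLocation to reach the last crystal.
; A fixed delay, rather than arrival, restores movement and ends the ability.
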(event `self.K2_ActivateAbility`
  (bind _character_movement (`self.Character Movement`))
  (bind _returnvalue (`Pawn.GetController` (`self.As BP Aura Character`)))
  ;[1 1 1] Set Initial Values for Variables
  (set `self.MouseHitLocation` (0.0 0.0 0.0))
  (set `self.AvatarActor` (`self.GetAvatarActorFromActorInfo`))
  (bind _asbp_aura_character (cast `/Game/Blueprints/Aura/BP_AuraCharacter` (`self.AvatarActor`)))
  (set `self.As BP Aura Character` _asbp_aura_character)
  (bind _ascombat_interface (cast `CombatInterface` (`self.AvatarActor`)))
  (`CombatInterface.UpdateFacingTarget` _ascombat_interface (`self.MouseHitLocation`))
  (`AbilityTask_WaitInputRelease.WaitInputRelease` false
    (:`then`
      (message `AuraPlayerInterface.ShowTravelArrow` (`self.AvatarActor`)))
    (:`OnRelease`
      (`|ExecutionSequence`
        (:`then_0`
          ;[1 1 1] Get the Display Arrow's Location, use this for Direction of Travel for consistency.
          (bind _returnvalue_2 (message `AuraPlayerInterface.GetArrowDisplayPoint` (`self.AvatarActor`)))
          (set `self.MouseHitLocation` _returnvalue_2))
        (:`then_1`
          ;[1 1 1] Hide the Direction Arrow and Play the animation montage to Start the Movement.
          (message `AuraPlayerInterface.HideTravelArrow` (`self.AvatarActor`))
          (`|PlayMontage` (`self.GetOwningComponentFromActorInfo` self) "/Game/Assets/Characters/Aura/Animations/Abilities/Lash/AM_Spin.AM_Spin" 1.0 0.0 "Default"
            (:`then`
              ;[0.936 0.5048 1] Play Ultimate Line
              (`GameplayStatics.PlaySoundAtLocation` "/Game/Assets/Sounds/Abilities/ArcaneLash/Cue_LashOut.Cue_LashOut" (`Actor.K2_GetActorLocation` (`self.AvatarActor`)) (struct) 1.0 1.0 1.0 null null null null)
              ;[1 1 1] For Each Spawned Crystal Get the Players
              (set `/Game/Blueprints/Aura/BP_AuraCharacter.bIsSpinning` true (`self.As BP Aura Character`))
              (bind _returnvalue_3 (`self.SpawnCrystals`))
              (bind _output_get (set `self.Spawned Crystals` _returnvalue_3))
              (set `self.IndexSize` (`KismetArrayLibrary.Array_Length` _output_get))
              (`|ExecutionSequence`
                (:`then_0`
                  ;[1 1 1] Set Move to Location to last Shard
                  (bind _result (`/Engine/EditorBlueprintResources/StandardMacros.DecrementInt` (`self.IndexSize`))
                    (:`  `
                      (set `self.CrystalMoveToLocation` (`Actor.K2_GetActorLocation` (`|GetArrayItem` (`self.Spawned Crystals`) _result))))))
                (:`then_1`
                  ;[1 1 1] Increase Speed to Get there quickly, utilize the Simple Move to function to move to target point
                  (bind _output_get_2 (set `self.Character Movement` (`Character.CharacterMovement` (`self.As BP Aura Character`))))
                  (set `CharacterMovementComponent.MaxWalkSpeed` (`self.WalkSpeedWhileSpinning`) _output_get_2)
                  (set `CharacterMovementComponent.MaxAcceleration` (`self.AccellerationWhileSpinning`) _output_get_2)
                  (`Controller.SetIgnoreMoveInput` _returnvalue true)
                  (`AIBlueprintHelperLibrary.SimpleMoveToLocation` _returnvalue (`self.CrystalMoveToLocation`)))
                (:`then_2`
                  ;[1 1 1] After  Short Delay, return Input and Movement to Normal.
                  (`KismetSystemLibrary.Delay` 1.5)
                  (`Controller.SetIgnoreMoveInput` (`Pawn.GetController` (`self.As BP Aura Character`)) false)
                  (set `CharacterMovementComponent.MaxWalkSpeed` (`self.DefaultWalkSpeed`) _character_movement)
                  (set `CharacterMovementComponent.MaxAcceleration` (`self.DefaultAccelleration`) _character_movement)
                  (set `/Game/Blueprints/Aura/BP_AuraCharacter.bIsSpinning` false (`self.As BP Aura Character`))
                  (`self.K2_EndAbility`))))))))))