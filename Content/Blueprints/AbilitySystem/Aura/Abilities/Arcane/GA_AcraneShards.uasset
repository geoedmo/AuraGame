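; Arcane Shards gameplay ability that erupts a level-scaled number of damaging shards around a targeted ground point.
; It shows a magic circle until input press, then applies a cast effect, faces the mouse target, plays a montage and waits for cast completion.
; After committing, a spawned point collection supplies ground points, and a looping timer triggers radial damage with upward knockback plus a gameplay cue at each, then ends the ability.
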(event `self.K2_ActivateAbility`
  ;[1 0.3957 0.4057] Clamp the Amount of Shards
  (set `self.NumShards` (`KismetMathLibrary.Clamp` (`self.GetAbilityLevel`) 1 (`self.MaxShards`)))
  ;[1 1 1] Setup Avatar Info Local Variable (Used a lot), and Wait Input Press
  (set `self.AvatarActor` (`self.GetAvatarActorFromActorInfo`))
  (`AbilityTask_WaitInputPress.WaitInputPress` false
    (:`then`
      ;[0.2317 1 0.8396] Ability Pre-Cast Setup, Play Montage and Wait for Key Press
      (message `AuraPlayerInterface.ShowMagicCircle` (`self.AvatarActor`) null))
    (:`OnPress`
      (`self.BP_ApplyGameplayEffectToOwner` "/Game/Blueprints/AbilitySystem/Aura/Abilities/Arcane/GE_ArcaneShards_Cast.GE_ArcaneShards_Cast_C")
      (bind (_asynctaskproxy _data) (`TargetDataUnderMouse.CreateTargetDataUnderMouse`)
        (:`ValidData`
          (set `self.Impact Point` (`.ImpactPoint` (`GameplayStatics.BreakHitResult` (`AbilitySystemBlueprintLibrary.GetHitResultFromTargetData` _data))))
          (`self.UpdateFacingTarget`)
          (`AbilityTask_PlayMontageAndWait.CreatePlayMontageAndWaitProxy` "None" (`self.AnimationMontage`) 1.0 "None" false
            (:`then`
              (`WaitCastTimeChange.WaitForCastCompletion` (`self.GetAbilitySystemComponentFromActorInfo`)
                (:`then`
                  ;[0.2486 1 0.4505] Things Not Waiting for Cast Animation
                  (message `CombatInterface.SetIsCasting` (`self.AvatarActor`) true)
                  (message `AuraPlayerInterface.HideMagicCircle` (`self.AvatarActor`)))
                (:`CastTimeEnd`
                  ;[0.8414 1 0.3404] Commit Ability, Spawn the Shard Nodes Actor, and Select the Amount of Shards to Spawn by Ability Level
                  (`self.K2_CommitAbility`)
                  (bind _returnvalue (`|SpawnActorFromClass` "/Game/Blueprints/AbilitySystem/Aura/Abilities/Arcane/BP_PointCollection.BP_PointCollection_C" (`KismetMathLibrary.MakeTransform` (`self.Impact Point`)) "Undefined" "MultiplyWithRoot" null null))
                  (bind _output_get (set `self.PointCollection` _returnvalue))
                  (set `self.GroundPoints` (`PointCollectionActor.GetGroundPoints` _output_get (`self.Impact Point`) (`self.NumShards`) (`KismetMathLibrary.RandomFloatInRange` 0.0 360.0)))
                  ;[0.8213 0.4828 1] Timer Event for Arcane Shards
                  (bind _returnvalue_2 (`KismetSystemLibrary.K2_SetTimerDelegate` (delegate `SpawnCrystals`) (`self.IntervalTime`) true))
                  (set `self.CrystalTimerHandle` _returnvalue_2)
                  (`self.SpawnCrystals`))))))))))

(event `SpawnCrystals`
  ;[1 0.3921 0.2317] Check Count Against Amount of Shards to Spawn, End Ability if False
  (if (< (`self.Count`) (`self.NumShards`))
    ;[0.5221 0.8374 1] Invidually Cast Arcane Shards Over Time (Interval Time)
    (set `self.CrystalSpawnLocation` (`SceneComponent.K2_GetComponentLocation` (`|GetArrayItem` (`self.GroundPoints`) (`self.Count`))))
    (bind _outoverlappingactors (`AuraAbilitySystemLibrary.GetLivePlayersWithinRadius` (`self.AvatarActor`) (`|MakeArray` (`self.AvatarActor`)) (`self.RadialDamageOuterRadius`) (`self.CrystalSpawnLocation`)))
    (set `self.LivePlayersInRadius` _outoverlappingactors)
    ;[0.5221 0.8374 1] For Each of the Live Players Hit
    (for _array_element (`self.LivePlayersInRadius`)
      ;[0.5221 0.8374 1] Make Damage Effect Params and Set Knockback Directions
      (set `self.TargetActor` _array_element)
      (`AuraAbilitySystemLibrary.ApplyDamageEffect` (`self.MakeDamageEffectParamsFromClassDefaults` (`self.TargetActor`) (`self.CrystalSpawnLocation`) true (- (`Actor.K2_GetActorLocation` (`self.TargetActor`)) (`self.CrystalSpawnLocation`)) false (0.0 0.0 0.0) true 45.0)))
    ;[0.5221 0.8374 1] Make Gameplay Cues and Increment Event Timer Count
    (`/Engine/EditorBlueprintResources/StandardMacros.IncrementInt` (`self.Count`)
      (:`  `
        (`GameplayCueFunctionLibrary.ExecuteGameplayCueOnActor` (`self.AvatarActor`) (struct :`TagName` "GameplayCue.ArcaneShards") (`AbilitySystemBlueprintLibrary.MakeGameplayCueParameters` 0.0 0.0 (struct) (struct) (struct) (struct) (struct) (`self.CrystalSpawnLocation`)))))
    (else
      ;[1 0.2682 0.3279] Wrap Up Abilities Odds and Ends, End Ability
      (`KismetSystemLibrary.K2_ClearAndInvalidateTimerHandle` (`self.CrystalTimerHandle`))
      (message `CombatInterface.SetIsCasting` (`self.AvatarActor`) false)
      (`Actor.K2_DestroyActor` (`self.PointCollection`))
      (`KismetSystemLibrary.Delay` 0.2)
      (`self.K2_EndAbility`))))

(fn `UpdateFacingTarget`
  (message `CombatInterface.UpdateFacingTarget` (`self.GetAvatarActorFromActorInfo`) (`self.Impact Point`)))