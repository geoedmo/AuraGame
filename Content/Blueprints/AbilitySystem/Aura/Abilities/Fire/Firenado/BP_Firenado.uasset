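; Firenado ability actor: a moving fire tornado that leaves a trail behind it.
; Timelines scale it up, drive a random yaw sweep with rising velocity, then shrink it and switch off its Niagara effect and capsule queries.
; Looping timers add trail points at its location and, after a delay, remove tail segments.
; The actor outlives its visual, destroying itself once the trail's spline points or collision spheres run out.
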(event `self.ReceiveBeginPlay`
  (set `self.DefaultScale` (`self.GetActorScale3D` self))
  (`self.SetActorScale3D` (0.0 0.0 0.0))
  (bind (_direction _scale) (`Timeline|Timeline`)
    (:`Update`
      (`self.SetScale` _scale _scale _scale))
    (:`Finished`
      (bind _returnvalue (`self.GetTrail`))
      (set `self.FireTrail` _returnvalue)
      (set `self.InterpA` (`KismetMathLibrary.RandomFloatInRange` 0.0 360.0))
      (set `self.InterpB` (`KismetMathLibrary.RandomFloatInRange` 0.0 360.0))
      (`self.TrailDrop`)
      (bind _returnvalue_2 (`KismetSystemLibrary.K2_SetTimerDelegate` (delegate `TrailDrop`) (`self.TrailDropTime`) true))
      (set `self.TrailTimerHandle` _returnvalue_2)
      ;[1 1 1] Remove Ticks of Trail at Intervals here ... TODO
      (bind _returnvalue_3 (`KismetSystemLibrary.K2_SetTimerDelegate` (delegate `CustomEvent`) (`self.Removal Interval`) true false (`self.Removal Start Delay`)))
      (set `self.TrailRemovalTimer` _returnvalue_3)
      (`self.TrailDrop`)
      (bind (_direction_2 _yaw) (`Timeline|Speedincrease`)
        (:`Update`
          ;[1 1 1] Lerp Between Two Random Yaw Rotations
          (`self.K2_SetActorRotation` (`KismetMathLibrary.MakeRotator` 0.0 0.0 (`KismetMathLibrary.Lerp` (`self.InterpA`) (`self.InterpB`) _yaw)))
          ;[1 1 1] Increase Projectile Speed Over Time
          (set `MovementComponent.Velocity` (+ (`MovementComponent.Velocity` (`self.ProjectileMovement`)) (`self.GetActorForwardVector`)) (`self.ProjectileMovement`)))
        (:`Finished`
          (`KismetSystemLibrary.K2_ClearAndInvalidateTimerHandle` (`self.TrailTimerHandle`))
          (bind (_direction_3 _scale_2) (`Timeline|Decrease Scale`)
            (:`Update`
              (`self.SetScale` _scale_2 _scale_2 _scale_2))
            (:`Finished`
              (`ActorComponent.Deactivate` (`self.NiagaraComponent`))
              (`SceneComponent.SetVisibility` (`self.NiagaraComponent`) false false)
              (`PrimitiveComponent.SetCollisionEnabled` (`self.DamageCapsule`) "PhysicsOnly"))))))))

(event `TrailDrop`
  (`self.AddToTrails` self (`self.K2_GetActorLocation`)))

(event `CustomEvent`
  ;[1 1 1] Remove Ticks of Trail at Intervals here ... TODO
  (bind _returnvalue (`self.CheckIfTrailIsZero`))
  (if _returnvalue
    (`self.RemoveTailSegment`)
    (else
      (`KismetSystemLibrary.K2_ClearAndInvalidateTimerHandle` (`self.TrailRemovalTimer`))
      (`self.K2_DestroyActor`))))

(fn `CheckIfTrailIsZero`
  (returns (ReturnValue :type Boolean))
  (bind _returnvalue (`AuraTrailSpline.GetCollisionSphereArray` (`self.FireTrail`)))
  (bind _returnvalue_2 (`AuraTrailSpline.GetSpline` (`self.FireTrail`)))
  (return (and (> (`SplineComponent.GetNumberOfSplinePoints` _returnvalue_2) 0) (> (`KismetArrayLibrary.Array_Length` _returnvalue) 0))))

(fn `SetScale`
  (params (Y :type "Float (double-precision)") (Z :type "Float (double-precision)") (X :type "Float (double-precision)"))
  (`self.SetActorScale3D` (* (`KismetMathLibrary.MakeVector` X Y Z) (`self.DefaultScale`))))

(fn `UserConstructionScript`)