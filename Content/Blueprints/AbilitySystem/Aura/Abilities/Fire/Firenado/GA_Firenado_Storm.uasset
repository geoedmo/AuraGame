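; Firenado Storm gameplay ability that spawns a group of firenado actors around a targeted ground point.
; Activation shows a magic circle; a press captures the cursor target, plays the montage and waits out the cast before committing.
; A point collection supplies ground locations, and a looping timer spawns damage-configured firenados one at a time.
; Finally, each firenado receives the group array and the ability ends; level-clamped NumShards goes unused, with NumPoints setting the count.
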(event `self.K2_ActivateAbility`
  ;[1 0.3957 0.4057] Clamp the Amount of Shards
  (set `self.NumShards` (`KismetMathLibrary.Clamp` (`self.GetAbilityLevel`) 1 4))
  ;[1 1 1] Setup Avatar Info Local Variable (Used a lot), and Wait Input Press
  (set `self.AvatarActor` (`self.GetAvatarActorFromActorInfo`))
  (`AbilityTask_WaitInputPress.WaitInputPress` false
    (:`then`
      ;[0.2317 1 0.8396] Ability Pre-Cast Setup, Play Montage and Wait for Key Press
      (message `AuraPlayerInterface.ShowMagicCircle` (`self.AvatarActor`) (`self.Decal Material`)))
    (:`OnPress`
      (`self.BP_ApplyGameplayEffectToOwner` "/Game/Blueprints/AbilitySystem/Aura/Abilities/Arcane/GE_ArcaneShards_Cast.GE_ArcaneShards_Cast_C")
      (bind (_asynctaskproxy _data) (`TargetDataUnderMouse.CreateTargetDataUnderMouse`)
        (:`ValidData`
          (set `self.Impact Point` (`.ImpactPoint` (`GameplayStatics.BreakHitResult` (`AbilitySystemBlueprintLibrary.GetHitResultFromTargetData` _data))))
          (`self.UpdateFacingTarget`)
          (`AbilityTask_PlayMontageAndWait.CreatePlayMontageAndWaitProxy` "None" (`self.AnimationMontage`) 1.0 "None" false
            (:`then`
              (`WaitCastTimeChange.WaitForCastCompletion` (`self.GetAbilitySystemComponentFromActorInfo`)
                (:`then`
                  ;[0.2486 1 0.4505] Things Not Waiting for Cast Animation
                  (message `CombatInterface.SetIsCasting` (`self.AvatarActor`) true)
                  (message `AuraPlayerInterface.HideMagicCircle` (`self.AvatarActor`)))
                (:`CastTimeEnd`
                  ;[0.8414 1 0.3404] Commit Ability, Spawn the Shard Nodes Actor, and Select the Amount of Shards to Spawn by Ability Level
                  (`self.K2_CommitAbility`)
                  (bind _returnvalue (`|SpawnActorFromClass` "/Game/Blueprints/AbilitySystem/Aura/Abilities/Arcane/BP_PointCollection.BP_PointCollection_C" (`KismetMathLibrary.MakeTransform` (`self.Impact Point`)) "Undefined" "MultiplyWithRoot" null null))
                  (bind _output_get (set `self.PointCollection` _returnvalue))
                  (set `self.GroundPoints` (`PointCollectionActor.GetGroundPoints` _output_get (`self.Impact Point`) (`self.Num Points`) (`KismetMathLibrary.RandomFloatInRange` 0.0 360.0)))
                  ;[0.8213 0.4828 1] Timer Event for Arcane Shards
                  (bind _returnvalue_2 (`KismetSystemLibrary.K2_SetTimerDelegate` (delegate `SpawnCrystals`) (`self.IntervalTime`) true))
                  (set `self.CrystalTimerHandle` _returnvalue_2)
                  (`self.SpawnCrystals`))))))))))

(event `SpawnCrystals`
  ;[1 0.3921 0.2317] Check Count Against Amount of Shards to Spawn, End Ability if False
  (if (< (`self.Count`) (`self.Num Points`))
    ;[0.5221 0.8374 1] Invidually Cast Arcane Shards Over Time (Interval Time)
    (bind _output_get (set `self.CrystalSpawnLocation` (`SceneComponent.K2_GetComponentLocation` (`|GetArrayItem` (`self.GroundPoints`) (`self.Count`)))))
    (bind _returnvalue (`|SpawnActorFromClass` "/Game/Blueprints/AbilitySystem/Aura/Abilities/Fire/Firenado/BP_Firenado.BP_Firenado_C" (`KismetMathLibrary.MakeTransform` (`KismetMathLibrary.MakeVector` (.x _output_get) (.y _output_get) (+ (.z _output_get) 2.0)) (`KismetMathLibrary.MakeRotator` 0.0 0.0 (`KismetMathLibrary.RandomFloatInRange` 0.0 360.0))) "AlwaysSpawn" "MultiplyWithRoot" (`self.AvatarActor`) null))
    ;[1 0.2703 0.2603] Set Damage Params
    (bind _output_get_2 (set `self.SpawnedFirenado` _returnvalue))
    (`AuraDamageEffectActor.SetDamageEffectParams` _output_get_2 (`self.MakeDamageEffectParamsFromClassDefaults` null))
    (`KismetArrayLibrary.Array_Add` (`self.SpawnedActors`) (`self.SpawnedFirenado`))
    (`/Engine/EditorBlueprintResources/StandardMacros.IncrementInt` (`self.Count`))
    (else
      ;[1 1 1] Add the Spawned Actors Array to Each Spawned Damage Effect Actor
      (for _array_element (`self.SpawnedActors`)
        (`AuraDamageEffectActor.SetArrayOfGroupedActors` _array_element (`self.SpawnedActors`)))
      ;[1 0.2682 0.3279] Wrap Up Abilities Odds and Ends, End Ability
      (`KismetSystemLibrary.K2_ClearAndInvalidateTimerHandle` (`self.CrystalTimerHandle`))
      (message `CombatInterface.SetIsCasting` (`self.AvatarActor`) false)
      (`Actor.K2_DestroyActor` (`self.PointCollection`))
      (`KismetSystemLibrary.Delay` 0.2)
      (`self.K2_EndAbility`))))

(fn `UpdateFacingTarget`
  (message `CombatInterface.UpdateFacingTarget` (`self.GetAvatarActorFromActorInfo`) (`self.Impact Point`)))