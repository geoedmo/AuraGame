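; Boomerang-style fireball actor for Aura's Fire Blast ability that flies out, returns and explodes.
; On the server, one timeline lerps it forward to an apex, then a second pulls it back toward the moving ReturnTarget.
; Within ExplodeDistance of that target, it calls OnHit, applies radial damage and 45-degree-pitched knockback to nearby live players except its owner, then destroys itself.
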(event `self.ReceiveBeginPlay`
  (`/Engine/EditorBlueprintResources/ActorMacros.Switch Has Authority`
    (:`Authority`
      (set `self.Location` (`self.K2_GetActorLocation`))
      (set `self.ForwardUnitVectorWithLength` (* (`self.GetActorForwardVector`) (`self.DistanceToTravel`)))
      (set `self.ApexLocation` (+ (`self.Location`) (`self.ForwardUnitVectorWithLength`)))
      (bind (_direction _traveldivision) (`Timeline|Timeline`)
        (:`Update`
          (`self.K2_SetActorLocation` (`KismetMathLibrary.VLerp` (`self.Location`) (`self.ApexLocation`) _traveldivision)))
        (:`Finished`
          (`self.Play Revese`))))))

(event `Play Revese`
  (bind _returnvalue (`self.GetOwner`))
  (bind (_returnvalue_x _returnvalue_y _returnvalue_z) (`self.OverridePitch`))
  (bind _array (`|MakeArray` _returnvalue))
  (`/Engine/EditorBlueprintResources/ActorMacros.Switch Has Authority`
    (:`Authority`
      (set `self.Aura` (`self.GetOwner`))
      (bind (_direction _backtoaura) (`Timeline|Timeline_0`)
        (:`Update`
          (bind _output_get (set `self.AuraLocation` (`self.K2_GetActorLocation` (`self.ReturnTarget`))))
          (`self.K2_SetActorLocation` (`KismetMathLibrary.VLerp` _output_get (`self.K2_GetActorLocation`) _backtoaura))
          (if (`self.SetExplodeDistance`)
            (`self.OnHit`)
            (`KismetArrayLibrary.Array_Add` _array self)
            (bind _outoverlappingactors (`AuraAbilitySystemLibrary.GetLivePlayersWithinRadius` _returnvalue _array (`self.QueryRadius`) (`self.K2_GetActorLocation`)))
            (for _array_element _outoverlappingactors
              (if (`KismetSystemLibrary.IsValid` _array_element)
                (`AuraAbilitySystemLibrary.SetTargetDamageEffectParamsASC` (`self.ExplosionDamageParams`) (`AbilitySystemBlueprintLibrary.GetAbilitySystemComponent` _array_element))
                (set `self.KnockbackDirection` (- (`self.K2_GetActorLocation` _array_element) (`self.K2_GetActorLocation`)))
                (`AuraAbilitySystemLibrary.SetIsRadialDamageEffectParams` (`self.ExplosionDamageParams`) true 50.0 (`self.QueryRadius`) (`self.K2_GetActorLocation`))
                ;[1 1 1] Add in Knockback and DeathImpluse Setters
                (`AuraAbilitySystemLibrary.SetKnockbackParams` (`self.ExplosionDamageParams`) (`KismetMathLibrary.MakeVector` _returnvalue_x _returnvalue_y _returnvalue_z))
                (`AuraAbilitySystemLibrary.SetDeathImpulseDirection` (`self.ExplosionDamageParams`) (`self.KnockbackDirection`))
                (`AuraAbilitySystemLibrary.ApplyDamageEffect` (`self.ExplosionDamageParams`))))
            (`self.K2_DestroyActor`)))))))

(fn `OverridePitch`
  (returns (ReturnValue_X :type "Float (double-precision)") (ReturnValue_Y :type "Float (double-precision)") (ReturnValue_Z :type "Float (double-precision)"))
  (bind (_returnvalue_roll _returnvalue_pitch _returnvalue_yaw) (`KismetMathLibrary.BreakRotator` (`KismetMathLibrary.Conv_VectorToRotator` (`self.KnockbackDirection`))))
  (bind (_returnvalue_x _returnvalue_y _returnvalue_z) (`KismetMathLibrary.BreakVector` (`KismetMathLibrary.Conv_RotatorToVector` (`KismetMathLibrary.MakeRotator` _returnvalue_roll 45.0 _returnvalue_yaw))))
  (return _returnvalue_x _returnvalue_y _returnvalue_z))

(fn `SetExplodeDistance`
  (returns (ReturnValue :type Boolean))
  (return (<= (`KismetMathLibrary.VSize` (- (`self.K2_GetActorLocation`) (`self.K2_GetActorLocation` (`self.ReturnTarget`)))) (`self.ExplodeDistance`))))

(fn `UserConstructionScript`)