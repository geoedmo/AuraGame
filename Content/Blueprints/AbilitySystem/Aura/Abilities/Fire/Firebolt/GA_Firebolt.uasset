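; GA_Firebolt is the gameplay ability for casting Firebolt, which launches projectiles from the avatar's weapon socket toward the target under the mouse.
; Activation applies a cast-time effect, captures the hit actor and location, turns the caster to face it and plays the cast montage.
; An async wait for cast completion then commits the ability and spawns projectiles with a homing target and pitch override.
; The ability ends after spawning or when the montage finishes or is interrupted.
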(event `self.K2_ActivateAbility`
  (`self.BP_ApplyGameplayEffectToOwner` "/Game/Blueprints/AbilitySystem/Aura/Abilities/Fire/Firebolt/GE_Firebolt_CastTime.GE_Firebolt_CastTime_C")
  (bind (_asynctaskproxy _data) (`TargetDataUnderMouse.CreateTargetDataUnderMouse`)
    (:`ValidData`
      (bind (_bblockinghit _binitialoverlap _time _distance _location _impactpoint _normal _impactnormal _physmat _hitactor) (`GameplayStatics.BreakHitResult` (`AbilitySystemBlueprintLibrary.GetHitResultFromTargetData` _data)))
      (set `self.HomingTarget` _hitactor)
      (set `self.ProjectTargetLocation` _location)
      (bind _ascombat_interface (cast `CombatInterface` (`self.GetAvatarActorFromActorInfo`)))
      (`CombatInterface.UpdateFacingTarget` _ascombat_interface (`self.ProjectTargetLocation`))
      (`AbilityTask_PlayMontageAndWait.CreatePlayMontageAndWaitProxy` "None" "/Game/Assets/Characters/Aura/Animations/Abilities/AM_Cast_Firebolt.AM_Cast_Firebolt"
        (:`then`
          (`WaitCastTimeChange.WaitForCastCompletion` (`self.GetAbilitySystemComponentFromActorInfo`)
            (:`CastTimeEnd`
              (`self.K2_CommitAbility`)
              (`self.SpawnProjectiles` (`self.ProjectTargetLocation`) (`BlueprintGameplayTagLibrary.MakeLiteralGameplayTag` (struct :`TagName` "CombatSocket.Weapon")) (`self.HomingTarget`) true 25.0)
              (`self.K2_EndAbility`))))
        (:`OnCompleted`
          (`self.K2_EndAbility` :!label _label))
        (:`OnBlendOut`
          (goto _label))
        (:`OnInterrupted`
          (goto _label))
        (:`OnCancelled`
          (goto _label))))))